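; Spline-based river actor that extends a parent WaterBody_BP0's reactive water along a path.
; The construction script builds spline meshes sized by point scale, with preview materials.
; At BeginPlay it passes the water body's heightfield textures and settings to dynamic materials, or repeatedly prints a warning if unattached.
; A Tick-fed gate and 0.2s delay periodically reposition the river capture and clip plane and update the materials' capture location.
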(event EventBeginPlay
  (bind _returnvalue (Actor|GetAttachParentActor))
  (Utilities|FlowControl|Delay 0.1)
  (if (Utilities|String|Contains (Utilities|GetObjectName _returnvalue) "WaterBody")
    (bind _aswater_body_bp0 (Utilities|Casting|CastToWaterBody_BP0 _returnvalue))
    (Variables|Default|SetRelatedWaterBody _aswater_body_bp0)
    (Utilities|FlowControl|Sequence
      (:then_0
        (Variables|Default|SetRiverCapture (Variables|/Game/_Marvelmaster_infinite_reactive_water_/Blueprints/WaterBody_BP0.WaterBody_BP0_C|GetRiverCaptureActor (Variables|Default|GetRelatedWaterBody)))
        (for _array_element (Variables|Default|GetSplineArray)
          (bind _returnvalue_2 (Rendering|Material|CreateDynamicMaterialInstance _array_element 0 (Variables|Default|GetRiverMaterial) "None" :!class /Script/Engine.PrimitiveComponent))
          (Utilities|Array|Add (Variables|Default|GetSplineMatArray) _returnvalue_2))
        (for _array_element_2 (Variables|Default|GetSplineMatArray)
          (Rendering|Material|SetTextureParameterValue _array_element_2 "HeightfieldNormal" (Variables|/Game/_Marvelmaster_infinite_reactive_water_/Blueprints/WaterBody_BP0.WaterBody_BP0_C|GetHeightfieldNormal (Variables|Default|GetRelatedWaterBody)))
          (Rendering|Material|SetTextureParameterValue _array_element_2 "Heightfield" (Variables|/Game/_Marvelmaster_infinite_reactive_water_/Blueprints/WaterBody_BP0.WaterBody_BP0_C|GetCurrentHeightMap (Variables|Default|GetRelatedWaterBody)))
          (Rendering|Material|SetScalarParameterValue _array_element_2 "SimulationDistance" (Variables|/Game/_Marvelmaster_infinite_reactive_water_/Blueprints/WaterBody_BP0.WaterBody_BP0_C|GetSimulation%20Distance (Variables|Default|GetRelatedWaterBody)) :!class /Script/Engine.MaterialInstanceDynamic))
        (for _array_element_3 (Variables|Default|GetSplineMatArray)
          (Rendering|Material|SetScalarParameterValue _array_element_3 "Rivermode" (Math|Conversions|ToFloat(Boolean) (Variables|/Game/_Marvelmaster_infinite_reactive_water_/Blueprints/WaterBody_BP0.WaterBody_BP0_C|GetSwitchToRiverMode (Variables|Default|GetRelatedWaterBody))) :!class /Script/Engine.MaterialInstanceDynamic)
          (Rendering|Material|SetScalarParameterValue _array_element_3 "RiverTiling" (Variables|Default|GetRiverTiling) :!class /Script/Engine.MaterialInstanceDynamic)))
      (:then_1
        (Utilities|FlowControl|Gate true) ; enters at Open
      ))
    (else
      (|PrintDebugInfo))))

(event Collision|EventActorBeginOverlap
  (params (OtherActor :type Actor%20Object%20Reference)))

(event EventTick
  (params (DeltaSeconds :type Float%20%28single-precision%29))
  (bind _relatedwaterbody (Variables|Default|GetRelatedWaterBody))
  (bind _relatedwaterbody_2 (Variables|Default|GetRelatedWaterBody))
  (bind _returnvalue (Transformation|GetActorLocation _relatedwaterbody))
  (bind _splinezloc (Variables|/Game/_Marvelmaster_infinite_reactive_water_/Blueprints/WaterBody_BP0.WaterBody_BP0_C|GetSplineZLoc _relatedwaterbody_2))
  (bind _z (Math|Vector|BreakVector _splinezloc))
  (Utilities|FlowControl|Gate true
    (:Exit
      (Utilities|FlowControl|Delay 0.2)
      (Transformation|SetActorLocation (Variables|Default|GetRiverCapture) (Math|Vector|MakeVector (.x _returnvalue) (.y _returnvalue) _z) false false)
      (Variables|/Script/Engine.SceneCaptureComponent2D|SetClipPlaneBase (Variables|/Game/_Marvelmaster_infinite_reactive_water_/Blueprints/WaterBody_BP0.WaterBody_BP0_C|GetSceneCaptureComponent2D _relatedwaterbody) (Math|Vector|MakeVector 0.0 0.0 (- _z (Variables|/Game/_Marvelmaster_infinite_reactive_water_/Blueprints/WaterBody_BP0.WaterBody_BP0_C|GetUnderWaterPrecision _relatedwaterbody))))
      (for _array_element (Variables|Default|GetSplineMatArray)
        (Rendering|Material|SetVectorParameterValue _array_element "CaptureLocation" (Variables|/Game/_Marvelmaster_infinite_reactive_water_/Blueprints/WaterBody_BP0.WaterBody_BP0_C|GetCaptureLocation (Variables|Default|GetRelatedWaterBody)) :!class /Script/Engine.MaterialInstanceDynamic)))))

(fn ConstructionScript
  (bind _spline (Variables|Default|GetSpline))
  (bind _spline_2 (Variables|Default|GetSpline))
  (for _index (range 0 (- (Spline|GetNumberOfSplinePoints (Variables|Default|GetSpline)) 2))
    (bind _returnvalue (AddComponent|AddSplineMeshComponent true))
    (Utilities|Array|Add (Variables|Default|GetSplineArray) _returnvalue)
    (Transformation|AttachComponentToComponent _returnvalue (Variables|Default|GetDefaultSceneRoot) "None" "KeepRelative" "KeepRelative" "KeepRelative" true)
    (Utilities|FlowControl|Sequence
      (:then_0
        (SplineMesh|SetStartandEnd _returnvalue (.Location (Spline|GetLocationandTangentatSplinePoint _spline _index "Local")) (.Tangent (Spline|GetLocationandTangentatSplinePoint _spline _index "Local")) (.Location (Spline|GetLocationandTangentatSplinePoint _spline (+ _index 1) "Local")) (.Tangent (Spline|GetLocationandTangentatSplinePoint _spline (+ _index 1) "Local")) true :!class /Script/Engine.SplineMeshComponent)
        ;[1 1 1] just for preview
        (for _array_element (Variables|Default|GetSplineArray)
          (bind _returnvalue_2 (Rendering|Material|CreateDynamicMaterialInstance _array_element 0 (Variables|Default|GetRiverMaterial) "None" :!class /Script/Engine.PrimitiveComponent))
          (Utilities|Array|Add (Variables|Default|GetSplineMatArray) _returnvalue_2)
          (for _array_element_2 (Variables|Default|GetSplineMatArray)
            (Rendering|Material|SetScalarParameterValue _array_element_2 "Rivermode" (Math|Conversions|ToFloat(Boolean) true) :!class /Script/Engine.MaterialInstanceDynamic)
            (Rendering|Material|SetScalarParameterValue _array_element_2 "RiverTiling" (Variables|Default|GetRiverTiling) :!class /Script/Engine.MaterialInstanceDynamic))
          ;[1 1 1] up and down do refresh on variable set
          (Transformation|AddActorLocalOffset "0, 0,0.010000" false false)
          (Transformation|AddActorLocalOffset "0, 0,-0.010000" false false)))
      (:then_1
        (Development|PrintString "Hello"))))
  (for (_array_element_3 _array_index) (Variables|Default|GetSplineArray)
    (SplineMesh|SetStartScale _array_element_3 (Math|Vector2D|MakeVector2D (.y (Spline|GetScaleatSplinePoint _spline_2 _array_index)) 1.0) true :!class /Script/Engine.SplineMeshComponent)
    (SplineMesh|SetEndScale _array_element_3 (Math|Vector2D|MakeVector2D (* (.y (Spline|GetScaleatSplinePoint _spline_2 _array_index)) 1.0) 1.0) true :!class /Script/Engine.SplineMeshComponent)
    (SplineMesh|SetEndScale _array_element_3 (Math|Vector2D|MakeVector2D (.y (Spline|GetScaleatSplinePoint _spline_2 (+ _array_index 1))) 1.0) true :!class /Script/Engine.SplineMeshComponent)
    (Development|PrintString "Hello")))